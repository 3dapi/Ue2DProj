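; BP_Enemy2 is an enemy actor that flies straight ahead while periodically shooting at the player.
; Tick moves it along its forward vector at Speed without sweeping, and destroys it once its accumulated lifetime reaches LifeTimeMax.
; A looping timer started on BeginPlay spawns BP_WeaponBullet at its location, rotated toward the player character's current position.
; InitTransform is an empty stub, and overlap is unhandled.
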(event EventBeginPlay
  (CallFunction|InitTransform)
  (Utilities|Time|SetTimerbyFunctionName 0 "OnEventFireBullet" 2.5 true))

(event Collision|EventActorBeginOverlap
  (params (OtherActor :type Actor%20Object%20Reference)))

(event EventTick
  (params (DeltaSeconds :type Float%20%28single-precision%29))
  (CallFunction|MoveForward DeltaSeconds)
  (bind _output_get (Variables|Default|SetlifeTimeStore (+ DeltaSeconds (Variables|Default|GetlifeTimeStore))))
  (if (>= _output_get (Variables|Default|GetlifeTimeMax))
    (Actor|DestroyActor)))

(event EventEndPlay
  (params (EndPlayReason :type EEndPlayReason%20Enum :default "Destroyed"))
  (Utilities|Time|ClearTimerbyFunctionName 0 "OnEventFireBullet"))

(fn ConstructionScript)

(fn InitTransform)

(fn MoveForward
  (params (deltaTime :type Float%20%28double-precision%29))
  (bind _returnvalue (Transformation|GetActorTransform))
  (Transformation|SetActorTransform (Math|Transform|MakeTransform (+ (* (Transformation|GetActorForwardVector) (* deltaTime (Variables|Default|Getspeed))) (.location _returnvalue)) (.rotation _returnvalue) (.scale _returnvalue))))

(fn OnEventFireBullet
  (Game|SpawnActorfromClass "/Game/Project/Asset/BP_WeaponBullet.BP_WeaponBullet_C" (Math|Transform|MakeTransform (Transformation|GetActorLocation) (Math|Rotator|MakeRotfromX (Math|Vector|Normalize (- (Transformation|GetActorLocation (Game|GetPlayerCharacter 0)) (Transformation|GetActorLocation))))) "Undefined" 0 0))