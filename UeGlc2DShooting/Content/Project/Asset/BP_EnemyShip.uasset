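; BP_EnemyShip is an enemy ship that flies straight along its forward vector, shoots at the player and destroys itself when its lifetime expires.
; Tick moves it by Speed without sweeping and accumulates time toward LifeTimeMax.
; A looping timer spawns BP_WeaponBullet aimed at the player in the XZ plane, skipped when the ship is below an X threshold or almost atop the player.
; InitTransform is an empty stub.
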(event EventBeginPlay
  (CallFunction|InitTransform)
  (Utilities|Time|SetTimerbyFunctionName 0 "OnEventFireBullet" 1.5 true))

(event Collision|EventActorBeginOverlap
  (params (OtherActor :type Actor%20Object%20Reference)))

(event EventTick
  (params (DeltaSeconds :type Float%20%28single-precision%29))
  (CallFunction|MoveForward DeltaSeconds)
  (bind _output_get (Variables|Default|SetlifeTimeStore (+ DeltaSeconds (Variables|Default|GetlifeTimeStore))))
  (if (>= _output_get (Variables|Default|GetlifeTimeMax))
    (Actor|DestroyActor)))

(event EventEndPlay
  (params (EndPlayReason :type EEndPlayReason%20Enum :default "Destroyed"))
  (Utilities|Time|ClearTimerbyFunctionName 0 "OnEventFireBullet"))

(fn ConstructionScript)

(fn InitTransform)

(fn MoveForward
  (params (deltaTime :type Float%20%28double-precision%29))
  (bind _returnvalue (Transformation|GetActorTransform))
  (Transformation|SetActorTransform (Math|Transform|MakeTransform (+ (* (Transformation|GetActorForwardVector) (* deltaTime (Variables|Default|Getspeed))) (.location _returnvalue)) (.rotation _returnvalue) (.scale _returnvalue))))

(fn OnEventFireBullet
  (bind _returnvalue (Game|GetPlayerCharacter 0))
  (bind _returnvalue_2 (Transformation|GetActorLocation))
  (bind _returnvalue_3 (Transformation|GetActorLocation))
  (bind _returnvalue_4 (Transformation|GetActorLocation _returnvalue))
  (bind _returnvalue_5 (Math|Vector|MakeVector (.x _returnvalue_2) 0.0 (.z _returnvalue_2)))
  (bind _returnvalue_6 (Math|Vector|MakeVector (.x _returnvalue_4) 0.0 (.z _returnvalue_4)))
  (bind _returnvalue_7 (- _returnvalue_6 _returnvalue_5))
  (if (and (>= (.X (Math|Vector|BreakVector _returnvalue_3)) -3e+02) (> (Math|Vector|VectorLengthSquared _returnvalue_7) 1.0))
    (Game|SpawnActorfromClass "/Game/Project/Asset/BP_WeaponBullet.BP_WeaponBullet_C" (Math|Transform|MakeTransform _returnvalue_3 (Math|Rotator|MakeRotfromX (Math|Vector|Normalize _returnvalue_7))) "Undefined" 0 0)))