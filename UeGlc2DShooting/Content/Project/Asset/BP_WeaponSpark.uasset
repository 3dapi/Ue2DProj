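; BP_WeaponSpark is a projectile for a 2D plane shooter that flies along its forward vector and expires after a maximum lifetime.
; Tick moves it by setting its transform without sweep and accumulates its age.
; When player-owned, overlapping an Enemy-tagged actor spawns a one-shot explosion flipbook, plays sound, destroys both actors and adds score through BP2D_GameInstance.
; The branch for non-player shots hitting PlayerPlane is empty, as is InitTransform.
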(event Custom|CustomEventFBPlayEnd
  (Actor|DestroyActor (stale Collision|EventActorBeginOverlap _returnvalue)))

(event EventBeginPlay
  (CallFunction|InitTransform))

(event EventTick
  (params (DeltaSeconds :type Float%20%28single-precision%29))
  (CallFunction|MoveForward DeltaSeconds)
  (bind _output_get (Variables|Default|SetlifeTimeStore (+ DeltaSeconds (Variables|Default|GetlifeTimeStore))))
  (if (>= _output_get (Variables|Default|GetlifeTimeMax))
    (Actor|DestroyActor)))

(event Collision|EventActorBeginOverlap
  (params (OtherActor :type Actor%20Object%20Reference))
  (if (and (Variables|Default|GetisOwnerPlayer) (Actor|ActorHasTag OtherActor "Enemy"))
    (bind _returnvalue (Game|SpawnActorfromClass "/Script/Paper2D.PaperFlipbookActor" (Math|Transform|MakeTransform (Transformation|GetActorLocation OtherActor)) "Undefined" 0 0))
    (Sprite|SetFlipbook (Variables|/Script/Paper2D.PaperFlipbookActor|GetRenderComponent _returnvalue) (Variables|Default|GeteffectExplosionFB))
    (EventDispatchers|AssignOnFinishedPlaying (Variables|/Script/Paper2D.PaperFlipbookActor|GetRenderComponent _returnvalue) (delegate Custom|CustomEventFBPlayEnd))
    (Actor|SetLifeSpan _returnvalue (+ (/ (Components|Animation|GetPlayRate (Variables|/Script/Paper2D.PaperFlipbookActor|GetRenderComponent _returnvalue)) (Class|PaperFlipbookComponent|GetFlipbookLength (Variables|/Script/Paper2D.PaperFlipbookActor|GetRenderComponent _returnvalue))) 0.0))
    (Components|Timeline|SetLooping (Variables|/Script/Paper2D.PaperFlipbookActor|GetRenderComponent _returnvalue) false)
    (Components|Timeline|PlayfromStart (Variables|/Script/Paper2D.PaperFlipbookActor|GetRenderComponent _returnvalue))
    (Audio|PlaySound2D "/Game/Project/Asset/Sound/Cue_explosion.Cue_explosion" 1.0 1.0 0.0 0 0)
    (Actor|DestroyActor OtherActor)
    (Actor|DestroyActor self)
    (bind _asbp2d_game_instance (Utilities|Casting|CastToBP2D_GameInstance (Game|GetGameInstance)))
    (Default|AddScore _asbp2d_game_instance 180)
    (elif (and (not (Variables|Default|GetisOwnerPlayer)) (Actor|ActorHasTag OtherActor "PlayerPlane"))
      _)))

(fn ConstructionScript)

(fn InitTransform)

(fn MoveForward
  (params (deltaTime :type Float%20%28double-precision%29))
  (bind _returnvalue (Transformation|GetActorTransform))
  (Transformation|SetActorTransform (Math|Transform|MakeTransform (+ (* (Transformation|GetActorForwardVector) (* deltaTime (Variables|Default|Getspeed))) (.location _returnvalue)) (.rotation _returnvalue) (.scale _returnvalue))))