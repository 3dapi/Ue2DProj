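; Projectile actor for plane weapons that flies along its forward vector at a set speed and destroys itself after a maximum lifetime.
; On overlap, only non-player-owned bullets react, and only to actors tagged PlayerPlane, applying damage and playing an explosion sound.
; The hit also spawns a one-shot Paper2D flipbook explosion, cleaned up on finish or by lifespan.
; The bullet is only hidden on hit, remaining until its lifetime expires.
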(event Custom|CustomEventFBPlayEnd
  (Actor|DestroyActor (stale Collision|EventActorBeginOverlap _returnvalue_2)))

(event EventBeginPlay
  (CallFunction|InitTransform))

(event EventTick
  (params (DeltaSeconds :type Float%20%28single-precision%29))
  (CallFunction|MoveForward DeltaSeconds)
  (bind _output_get (Variables|Default|SetlifeTimeStore (+ DeltaSeconds (Variables|Default|GetlifeTimeStore))))
  (if (>= _output_get (Variables|Default|GetlifeTimeMax))
    (Actor|DestroyActor)))

(event Collision|EventActorBeginOverlap
  (params (OtherActor :type Actor%20Object%20Reference))
  (bind _returnvalue (Transformation|GetActorLocation OtherActor))
  (if (and (not (Variables|Default|GetisOwnerPlayer)) (Actor|ActorHasTag OtherActor "PlayerPlane"))
    (bind _returnvalue_2 (Game|SpawnActorfromClass "/Script/Paper2D.PaperFlipbookActor" (Math|Transform|MakeTransform (Math|Vector|MakeVector (.x _returnvalue) (+ (.y _returnvalue) 1e+01) (.z _returnvalue))) "Undefined" 0 0))
    (Sprite|SetFlipbook (Variables|/Script/Paper2D.PaperFlipbookActor|GetRenderComponent _returnvalue_2) (Variables|Default|GeteffectExplosionFB))
    (EventDispatchers|AssignOnFinishedPlaying (Variables|/Script/Paper2D.PaperFlipbookActor|GetRenderComponent _returnvalue_2) (delegate Custom|CustomEventFBPlayEnd))
    (Actor|SetLifeSpan _returnvalue_2 (+ (/ (Components|Animation|GetPlayRate (Variables|/Script/Paper2D.PaperFlipbookActor|GetRenderComponent _returnvalue_2)) (Class|PaperFlipbookComponent|GetFlipbookLength (Variables|/Script/Paper2D.PaperFlipbookActor|GetRenderComponent _returnvalue_2))) 1e+01))
    (Components|Timeline|SetLooping (Variables|/Script/Paper2D.PaperFlipbookActor|GetRenderComponent _returnvalue_2) false)
    (Components|Timeline|PlayfromStart (Variables|/Script/Paper2D.PaperFlipbookActor|GetRenderComponent _returnvalue_2))
    (Audio|PlaySound2D "/Game/Project/Asset/Sound/Cue_explosion.Cue_explosion" 1.0 1.0 0.0 0 0)
    (Game|Damage|ApplyDamage OtherActor (Variables|Default|Getdamage) 0 self)
    (Rendering|SetActorHiddenInGame self true)))

(fn ConstructionScript)

(fn InitTransform)

(fn MoveForward
  (params (deltaTime :type Float%20%28double-precision%29))
  (bind _returnvalue (Transformation|GetActorTransform))
  (Transformation|SetActorTransform (Math|Transform|MakeTransform (+ (* (Transformation|GetActorForwardVector) (* deltaTime (Variables|Default|Getspeed))) (.location _returnvalue)) (.rotation _returnvalue) (.scale _returnvalue))))