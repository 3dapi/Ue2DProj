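; Enemy spawner for a side-view 2D game that keeps spawning enemies ahead of the player.
; On BeginPlay it reads the difficulty from BP2D_GameInstance and starts a looping timer, with shorter intervals for higher options, which is cleared on EndPlay.
; Each tick of the timer randomly picks one of three enemy classes, places it at a random X/Z offset from the player on the Y=0 plane and randomizes its speed.
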(event EventBeginPlay
  (CallFunction|SetupGameInstance)
  (CallFunction|SelectGameDifficult))

(event Collision|EventActorBeginOverlap
  (params (OtherActor :type Actor%20Object%20Reference)))

(event EventTick
  (params (DeltaSeconds :type Float%20%28single-precision%29)))

(event EventEndPlay
  (params (EndPlayReason :type EEndPlayReason%20Enum :default "Destroyed"))
  (Utilities|Time|ClearTimerbyFunctionName 0 "OnEventSpawnEnemyShip"))

(fn ConstructionScript)

(fn OnEventSpawnEnemyShip
  (bind _returnvalue (Game|GetPlayerCharacter 0))
  (bind _returnvalue_2 (Transformation|GetActorLocation _returnvalue))
  (bind _returnvalue_3 (+ (.z _returnvalue_2) 2.4e+02))
  (bind _returnvalue_4 (+ (.z _returnvalue_2) -2.4e+02))
  (bind _returnvalue_5 (+ (.x _returnvalue_2) 7e+02))
  (bind _returnvalue_6 (+ (.x _returnvalue_2) 1.1e+03))
  (bind _returnvalue_7 (Math|Random|RandomFloatinRange _returnvalue_4 _returnvalue_3))
  (bind _returnvalue_8 (Math|Random|RandomFloatinRange _returnvalue_5 _returnvalue_6))
  (bind _returnvalue_9 (Math|Vector|MakeVector _returnvalue_8 0.0 _returnvalue_7))
  (bind _returnvalue_10 (Math|Transform|MakeTransform _returnvalue_9 "0.000000,180.000000,0.000000"))
  (switch int (Math|Random|RandomIntegerinRange 0 2)
    (:0
      (bind _returnvalue_11 (Game|SpawnActorfromClass "/Game/Project/Asset/BP_EnemyShip.BP_EnemyShip_C" _returnvalue_10 "Undefined" 0 0))
      (Utilities|IsValid _returnvalue_11
        (:Is%20Valid
          (Variables|/Game/Project/Asset/BP_EnemyShip.BP_EnemyShip_C|Setspeed _returnvalue_11 (Math|Random|RandomFloatinRange 2.5e+02 5.4e+02)))))
    (:1
      (bind _returnvalue_12 (Game|SpawnActorfromClass "/Game/Project/Asset/BP_Enemy1.BP_Enemy1_C" _returnvalue_10 "Undefined" 0 0))
      (Utilities|IsValid _returnvalue_12
        (:Is%20Valid
          (Variables|/Game/Project/Asset/BP_Enemy1.BP_Enemy1_C|Setspeed _returnvalue_12 (Math|Random|RandomFloatinRange 2.5e+02 5.4e+02)))))
    (:2
      (bind _returnvalue_13 (Game|SpawnActorfromClass "/Game/Project/Asset/BP_Enemy2.BP_Enemy2_C" _returnvalue_10 "Undefined" 0 0))
      (Utilities|IsValid _returnvalue_13
        (:Is%20Valid
          (Variables|/Game/Project/Asset/BP_Enemy2.BP_Enemy2_C|Setspeed _returnvalue_13 (Math|Random|RandomFloatinRange 2.5e+02 5.4e+02)))))))

(fn SetupGameInstance
  (bind _asbp2d_game_instance (Utilities|Casting|CastToBP2D_GameInstance (Game|GetGameInstance)))
  (Variables|Default|SetgameInstance _asbp2d_game_instance))

(fn SelectGameDifficult
  (bind _returnvalue (Math|Float|MakeLiteralFloat 0.4))
  (bind _returnvalue_2 (Math|Float|MakeLiteralFloat 1.1))
  (bind _returnvalue_3 (Math|Float|MakeLiteralFloat 0.7))
  (bind _gameinstance (Variables|Default|GetgameInstance))
  (bind _prj_gamedifficult (Variables|/Game/Project/Common/BP2D_GameInstance.BP2D_GameInstance_C|Getprj_gameDifficult _gameinstance))
  (bind _returnvalue_4 (Utilities|Select :Index _prj_gamedifficult :Option%200 _returnvalue_2 :Option%201 _returnvalue_3 :Option%202 _returnvalue))
  (Development|PrintString (Utilities|String|ToString(Float) _returnvalue_4))
  (Utilities|Time|SetTimerbyFunctionName 0 "OnEventSpawnEnemyShip" _returnvalue_4 true))