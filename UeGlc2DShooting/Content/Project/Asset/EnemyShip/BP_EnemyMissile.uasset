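; Enemy missile actor that flies straight along its forward vector.
; Each Tick, MoveForward offsets its location by forward vector, Speed and delta time, keeping rotation and scale and setting the transform without sweep.
; On BeginPlay, InitTransform only prints the actor's rotation and a zero vector as debug output, despite its name.
; It has no overlap, damage or lifetime logic.
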(event EventBeginPlay
  (CallFunction|InitTransform))

(event Collision|EventActorBeginOverlap
  (params (OtherActor :type Actor%20Object%20Reference)))

(event EventTick
  (params (DeltaSeconds :type Float%20%28single-precision%29))
  (CallFunction|MoveForward DeltaSeconds))

(fn ConstructionScript)

(fn InitTransform
  (Development|PrintString (Utilities|String|ToString(Rotator) (.rotation (Transformation|GetActorTransform))))
  (Development|PrintString (Utilities|String|ToString(Vector) "0, 0, 0")))

(fn MoveForward
  (params (deltaTime :type Float%20%28double-precision%29))
  (bind _returnvalue (Transformation|GetActorTransform))
  (Transformation|SetActorTransform (Math|Transform|MakeTransform (+ (* (Transformation|GetActorForwardVector) (* deltaTime (Variables|Default|Getspeed))) (.location _returnvalue)) (.rotation _returnvalue) (.scale _returnvalue))))