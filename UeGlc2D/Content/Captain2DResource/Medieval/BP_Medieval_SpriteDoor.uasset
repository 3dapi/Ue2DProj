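; BP_Medieval_SpriteDoor is a 2D sprite door that ends the level when an actor overlaps it.
; On any overlap, it casts to BP2D_GameInstance, calls IsSuccessPlay, swaps its sprite to DoorOpen, waits briefly, then opens LEVEL2D_PlayEnd.
; A debug print reporting whether the sprite swap succeeded follows the level-open call.
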(event EventBeginPlay)

(event Collision|EventActorBeginOverlap
  (params (OtherActor :type Actor%20Object%20Reference))
  (bind _asbp2d_game_instance (Utilities|Casting|CastToBP2D_GameInstance (Game|GetGameInstance)))
  (Default|IsSuccessPlay _asbp2d_game_instance)
  (bind _returnvalue (Rendering|Components|Sprite|SetSprite (Variables|Default|GetRenderComponent) (Variables|Default|GetdoorOpen)))
  (Utilities|FlowControl|Delay 2.0)
  (Game|OpenLevel(byName) "LEVEL2D_PlayEnd")
  (if _returnvalue
    (Development|PrintString "DoorOpen success")
    (else
      (Development|PrintString "DoorOpen failed"))))

(event EventTick
  (params (DeltaSeconds :type Float%20%28single-precision%29)))

(event Collision|EventHit
  (params (MyComp :type Primitive%20Component%20Object%20Reference) (Other :type Actor%20Object%20Reference) (OtherComp :type Primitive%20Component%20Object%20Reference) (bSelfMoved :type Boolean) (HitLocation :type Vector :default "0, 0, 0") (HitNormal :type Vector :default "0, 0, 0") (NormalImpulse :type Vector :default "0, 0, 0") (Hit :type Hit%20Result%20Structure%20%28by%20ref%29)))

(fn ConstructionScript)