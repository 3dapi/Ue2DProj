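; BP_HeroLady_zd is a PaperZD 2D side-scrolling player character that moves along world X, jumps and performs two attacks.
; Enhanced Input from IMC_2D drives movement, flips control yaw to face the travel direction, and triggers attacks through animation node jumps.
; LadyAnim2D_BP anim events feed OnAnimEvent, which spawns a different explosion actor per attack ahead of the sprite.
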(event Custom|CustomAnimNoti
  (params (eventType :type String) (arg1 :type String) (arg2 :type Integer))
  (CallFunction|OnAnimEvent eventType arg1 arg2))

(event Input|EnhancedActionEvents|EnhancedInputActionIA_2DJump
  (params (ActionValue :type Boolean) (ElapsedSeconds :type Float%20%28double-precision%29) (TriggeredSeconds :type Float%20%28double-precision%29) (InputAction :type Input%20Action%20Object%20Reference :default "/Game/Project/input/IA_2DJump.IA_2DJump"))
  (:Started
    (Character|Jump))
  (:Completed
    (Character|StopJumping)))

(event Input|EnhancedActionEvents|EnhancedInputActionIA_2DMove
  (params (ActionValue :type Float%20%28double-precision%29) (ElapsedSeconds :type Float%20%28double-precision%29) (TriggeredSeconds :type Float%20%28double-precision%29) (InputAction :type Input%20Action%20Object%20Reference :default "/Game/Project/input/IA_2DMove.IA_2DMove"))
  (:Triggered
    (Pawn|Input|AddMovementInput "1.000000,0.000000,0.000000" ActionValue false)
    (Math|Float|CompareFloat ActionValue 0.0
      (:>
        (Pawn|SetControlRotation (Pawn|GetController) (Math|Rotator|MakeRotator 0.0 0.0 0.0)))
      (:<
        (Pawn|SetControlRotation (Pawn|GetController) (Math|Rotator|MakeRotator 0.0 0.0 1.8e+02))))))

(event Input|EnhancedActionEvents|EnhancedInputActionIA_2DAttack1
  (params (ActionValue :type Boolean) (ElapsedSeconds :type Float%20%28double-precision%29) (TriggeredSeconds :type Float%20%28double-precision%29) (InputAction :type Input%20Action%20Object%20Reference :default "/Game/Project/input/IA_2DAttack1.IA_2DAttack1"))
  (:Started
    (CallFunction|JumpAnimNode "ATTACK1")))

(event Input|EnhancedActionEvents|EnhancedInputActionIA_2DAttack2
  (params (ActionValue :type Boolean) (ElapsedSeconds :type Float%20%28double-precision%29) (TriggeredSeconds :type Float%20%28double-precision%29) (InputAction :type Input%20Action%20Object%20Reference :default "/Game/Project/input/IA_2DAttack2.IA_2DAttack2"))
  (:Started
    (CallFunction|JumpAnimNode "ATTACK2")))

(event EventBeginPlay
  (CallFunction|InitInput)
  (bind _aslady_anim_2d_bp (Utilities|Casting|CastToLadyAnim2D_BP (Variables|/Script/PaperZD.PaperZDAnimationComponent|GetAnimInstance (Variables|Default|GetAnimationComponent))))
  (EventDispatchers|BindEventtoAnimEvent _aslady_anim_2d_bp (delegate Custom|CustomAnimNoti)))

(event Collision|EventActorBeginOverlap
  (params (OtherActor :type Actor%20Object%20Reference)))

(fn ConstructionScript)

(fn InitInput
  (bind _as플레이어_컨트롤러 (Utilities|Casting|CastToPlayerController (Pawn|GetController)))
  (Input|AddMappingContext (PlayerController|LocalPlayerSubsystems|GetEnhancedInputLocalPlayerSubsystem _as플레이어_컨트롤러) "/Game/Project/input/IMC_2D.IMC_2D" 0 "(bIgnoreAllPressedKeysUntilRelease=True,bForceImmediately=False)"))

(fn OnAnimEvent
  (params (eventType :type String) (arg1 :type String) (arg2 :type Integer))
  (bind _returnvalue (CallFunction|LocationatForward 1.4e+02))
  (bind _returnvalue_2 (Math|Transform|MakeTransform _returnvalue))
  (switch string eventType
    (:AnimNoti
      (switch string arg1
        (:Attack1
          (Game|SpawnActorfromClass "/Game/StarterContent/Blueprints/Blueprint_Effect_Explosion.Blueprint_Effect_Explosion_C" _returnvalue_2 "Undefined" 0 0))
        (:Attack2
          (Game|SpawnActorfromClass "/Game/Project/Asset/Effect/BP_FBExplosion.BP_FBExplosion_C" _returnvalue_2 "Undefined" 0 0))))))

(fn JumpAnimNode
  (params (jumpName :type Name))
  (Class|PaperZDAnimInstance|JumptoNode (Variables|/Script/PaperZD.PaperZDAnimationComponent|GetAnimInstance (Variables|Default|GetAnimationComponent)) jumpName "None"))

(fn LocationatForward
  (params (forwardDist :type Float%20%28double-precision%29))
  (return (+ (* (Math|Vector|GetForwardVector (Variables|Default|GetSprite)) forwardDist) (Transformation|GetWorldLocation (Variables|Default|GetSprite)))))