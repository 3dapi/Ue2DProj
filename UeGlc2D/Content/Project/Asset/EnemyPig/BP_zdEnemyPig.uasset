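; BP_zdEnemyPig is a 2D enemy pig that attacks and damages the player's hero.
; While IsAttacking is set, Tick jumps its animation instance to the ATTACK1 node every frame.
; BeginPlay binds animation notifies to OnAnimEvent, which sends a HitDamage message to the player's BP2D_HeroLadyZd pawn.
; The event type and argument switches are disconnected, so every notify deals damage, with no range or overlap check.
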(event Custom|CustomAnimNotify
  (params (eventType :type String) (arg1 :type String) (arg2 :type Integer))
  (CallFunction|OnAnimEvent eventType arg1 arg2))

(event EventBeginPlay
  (bind _asenemy_pig_anim_2d_bp (Utilities|Casting|CastToEnemyPigAnim2D_BP (Variables|/Script/PaperZD.PaperZDAnimationComponent|GetAnimInstance (Variables|Default|GetAnimationComponent))))
  (EventDispatchers|AssignAnimEvent _asenemy_pig_anim_2d_bp (delegate Custom|CustomAnimNotify)))

(event Collision|EventActorBeginOverlap
  (params (OtherActor :type Actor%20Object%20Reference)))

(event EventTick
  (params (DeltaSeconds :type Float%20%28single-precision%29))
  (if (Variables|Default|GetisAttacking)
    (Class|PaperZDAnimInstance|JumptoNode (Variables|/Script/PaperZD.PaperZDAnimationComponent|GetAnimInstance (Variables|Default|GetAnimationComponent)) "ATTACK1" "None")))

(fn ConstructionScript)

(fn OnAnimEvent
  (params (eventType :type String) (arg1 :type String) (arg2 :type Integer))
  (bind _asbp2d_hero_lady_zd (Utilities|Casting|CastToBP2D_HeroLadyZd (Pawn|GetControlledPawn (Game|GetPlayerController 0))))
  (Default|OnMessage _asbp2d_hero_lady_zd "HitDamage" "" (Variables|Default|GethitDamage)))