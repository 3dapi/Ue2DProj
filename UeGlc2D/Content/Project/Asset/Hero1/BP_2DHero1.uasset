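; BP_2DHero1 is a side-scrolling 2D hero character with flipbook sprites, controlled through Enhanced Input.
; On BeginPlay it adds the IMC_2D mapping context, whose actions drive jumping and movement along the X axis.
; Move direction flips the controller yaw between facing right and left.
; Each Tick, UpdateAnimation picks idle, run, rise or landing flipbooks from ground state and velocity.
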(event Input|EnhancedActionEvents|EnhancedInputActionIA_2DJump
  (params (ActionValue :type Boolean) (ElapsedSeconds :type Float%20%28double-precision%29) (TriggeredSeconds :type Float%20%28double-precision%29) (InputAction :type Input%20Action%20Object%20Reference :default "/Game/Project/input/IA_2DJump.IA_2DJump"))
  (:Started
    (Character|Jump))
  (:Completed
    (Character|StopJumping)))

(event Input|EnhancedActionEvents|EnhancedInputActionIA_2DMove
  (params (ActionValue :type Float%20%28double-precision%29) (ElapsedSeconds :type Float%20%28double-precision%29) (TriggeredSeconds :type Float%20%28double-precision%29) (InputAction :type Input%20Action%20Object%20Reference :default "/Game/Project/input/IA_2DMove.IA_2DMove"))
  (:Triggered
    (Pawn|Input|AddMovementInput "1.000000,0.000000,0.000000" ActionValue false)
    (Math|Float|CompareFloat ActionValue 0.0
      (:>
        (Pawn|SetControlRotation (Pawn|GetController) (Math|Rotator|MakeRotator 0.0 0.0 0.0)))
      (:<
        (Pawn|SetControlRotation (Pawn|GetController) (Math|Rotator|MakeRotator 0.0 0.0 1.8e+02))))))

(event EventBeginPlay
  (CallFunction|InitInput))

(event Collision|EventActorBeginOverlap
  (params (OtherActor :type Actor%20Object%20Reference)))

(event EventTick
  (params (DeltaSeconds :type Float%20%28single-precision%29))
  (CallFunction|UpdateAnimation))

(fn ConstructionScript)

(fn UpdateAnimation
  ;[0.05208 0.05208 0.05208 1 11] 코멘트
  (if (AI|Components|NavMovement|IsMovingonGround (Variables|Character|GetCharacterMovement))
    (if (> (Math|Vector|VectorLengthSquared (Transformation|GetVelocity)) 0.0)
      (Sprite|SetFlipbook (Variables|Default|GetSprite) (Variables|Animation|GetflipbookRun))
      (else
        (Sprite|SetFlipbook (Variables|Default|GetSprite) (Variables|Animation|GetflipbookIdle))))
    (elif (>= (.z (Transformation|GetVelocity)) -1e+02)
      (Sprite|SetFlipbook (Variables|Default|GetSprite) (Variables|Animation|GetflipbookJumpRise))
      (else
        (Sprite|SetFlipbook (Variables|Default|GetSprite) (Variables|Animation|GetflipbookJumpLand))))))

(fn InitInput
  (bind _as플레이어_컨트롤러 (Utilities|Casting|CastToPlayerController (Pawn|GetController)))
  (Input|AddMappingContext (PlayerController|LocalPlayerSubsystems|GetEnhancedInputLocalPlayerSubsystem _as플레이어_컨트롤러) "/Game/Project/input/IMC_2D.IMC_2D" 0 "(bIgnoreAllPressedKeysUntilRelease=True,bForceImmediately=False)"))