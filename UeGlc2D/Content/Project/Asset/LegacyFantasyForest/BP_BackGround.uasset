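; Background actor for the LegacyFantasyForest scene that follows the player and displays a time-driven sprite material.
; BeginPlay creates a dynamic instance of MTL_CustomSprite and stores it as MtlBackgroundUV.
; Each Tick writes game time to its ParamTime parameter and reapplies the material to RenderComponent.
; Tick also moves the actor to the player character's X and Z, holding Y at DeepY for depth.
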(event EventBeginPlay
  (bind _returnvalue (Rendering|Material|CreateDynamicMaterialInstance "/Game/Project/Asset/MTL_CustomSprite.MTL_CustomSprite" "None" "None" :!class /Script/Engine.KismetMaterialLibrary))
  (Variables|Default|SetmtlBackgroundUV _returnvalue))

(event Collision|EventActorBeginOverlap
  (params (OtherActor :type Actor%20Object%20Reference)))

(event EventTick
  (params (DeltaSeconds :type Float%20%28single-precision%29))
  (bind _returnvalue (Game|GetPlayerCharacter 0))
  (bind _returnvalue_2 (Transformation|GetActorLocation _returnvalue))
  (bind (_x _y _z) (Math|Vector|BreakVector _returnvalue_2))
  (Utilities|FlowControl|Sequence
    (:then_0
      (Rendering|Material|SetScalarParameterValue (Variables|Default|GetmtlBackgroundUV) "ParamTime" (Utilities|Time|GetGameTimeinSeconds) :!class /Script/Engine.MaterialInstanceDynamic)
      (Rendering|Material|SetMaterial (Variables|Default|GetRenderComponent) 0 (Variables|Default|GetmtlBackgroundUV)))
    (:then_1
      (Transformation|SetActorLocation (Math|Vector|MakeVector _x (Variables|Default|GetdeepY) _z) false false))))

(fn ConstructionScript)